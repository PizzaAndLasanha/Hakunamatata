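; Cave building block that lays a chain of spline mesh segments along its spline to form a cave in the level.
; The construction script derives section length from the actor's X scale, then BuildCave adds one X-forward mesh component per whole section, leaving any shorter remainder uncovered.
; Each segment takes its endpoints and tangents from the spline, with tangent size clamped to the section length.
; The event graph has no active logic.
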(fn `BuildCave`
  (bind _spline (`self.Spline`))
  (bind _spline_2 (`self.Spline`))
  (for _index (range (`KismetMathLibrary.FFloor` (/ (`SplineComponent.GetSplineLength` (`self.Spline`)) (`self.SectionLength`))))
    (bind _returnvalue (`AddComponent|NODE_AddSplineMeshComponent-0`))
    (`SplineMeshComponent.SetForwardAxis` _returnvalue "X" true)
    (bind _returnvalue_2 (* _index (`self.SectionLength`)))
    (bind _returnvalue_3 (* (+ _index 1) (`self.SectionLength`)))
    (`SplineMeshComponent.SetStartAndEnd` _returnvalue (`SplineComponent.GetLocationAtDistanceAlongSpline` _spline_2 _returnvalue_2 "Local") (`KismetMathLibrary.ClampVectorSize` (`SplineComponent.GetTangentAtDistanceAlongSpline` _spline_2 _returnvalue_2 "Local") 0.0 (`self.SectionLength`)) (`SplineComponent.GetLocationAtDistanceAlongSpline` _spline _returnvalue_3 "Local") (`KismetMathLibrary.ClampVectorSize` (`SplineComponent.GetTangentAtDistanceAlongSpline` _spline _returnvalue_3 "Local") 0.0 (`self.SectionLength`)) true)))

(fn `UserConstructionScript`
  (bind _returnvalue_x (`KismetMathLibrary.BreakVector` (`self.GetActorScale3D`)))
  (set `self.SectionLength` (* _returnvalue_x 379.0))
  (`self.BuildCave`))