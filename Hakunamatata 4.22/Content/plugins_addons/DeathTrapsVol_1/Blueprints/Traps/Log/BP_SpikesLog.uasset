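; BP_SpikesLog is a spiked log trap actor that damages the player.
; When its DamageCollision component begins overlapping the first player pawn, it applies the Damage value to that pawn and ignores all other actors.
; The log mesh's hit event is empty, and a CauseDamage call on that mesh is left unconnected, so physical hits deal no damage here.
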(event `self.SM_Log.OnComponentHit`
  (params (HitComponent :type "PrimitiveComponent Object Reference") (OtherActor :type "Actor Object Reference") (OtherComp :type "PrimitiveComponent Object Reference") (NormalImpulse :type "Vector Structure") (Hit :type "HitResult Structure (by ref)"))
  ;[1 1 1] Cause damage by hit
)

(event `self.DamageCollision.OnComponentBeginOverlap`
  (params (OverlappedComponent :type "PrimitiveComponent Object Reference") (OtherActor :type "Actor Object Reference") (OtherComp :type "PrimitiveComponent Object Reference") (OtherBodyIndex :type Integer) (bFromSweep :type Boolean) (SweepResult :type "HitResult Structure (by ref)"))
  (if (== OtherActor (`GameplayStatics.GetPlayerPawn` 0))
    (`GameplayStatics.ApplyDamage` OtherActor (`self.damage`))))

(fn `UserConstructionScript`
  (`parent.UserConstructionScript`))