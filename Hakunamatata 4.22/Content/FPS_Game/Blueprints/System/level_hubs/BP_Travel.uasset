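; BP_Travel is a level-hub travel point that hands destination details to the game instance when interacted with.
; On interaction it calls LastKnownLocation on World_GameInstance with the map to load, the Arrow's facing, whether the current level is "main", and loading screen texture and text.
; The level load itself is not in this Blueprint, and its overlap events only cast to BP_CharacterBase with no further action.
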(event `self.ReceiveActorBeginOverlap`
  (params (OtherActor :type "Actor Object Reference"))
  (cast `/Game/ThirdPersonBP/BP_CharacterBase` OtherActor))

(event `self.ReceiveActorEndOverlap`
  (params (OtherActor :type "Actor Object Reference"))
  (cast `/Game/ThirdPersonBP/BP_CharacterBase` OtherActor))

(event `/Game/FPS_Game/Blueprints/System/BPI_Interact.BPI_Interaction`
  (bind _returnvalue (`GameplayStatics.GetCurrentLevelName` true))
  (bind _asworld_game_instance (cast `/Game/FPS_Game/Blueprints/System/level_hubs/World_GameInstance` (`GameplayStatics.GetGameInstance`)))
  (`/Game/FPS_Game/Blueprints/System/level_hubs/World_GameInstance.LastKnownLocation` _asworld_game_instance (`self.MapToLoad`) (`SceneComponent.K2_GetComponentRotation` (`self.Arrow`)) (`KismetStringLibrary.EqualEqual_StrStr` _returnvalue "main") (`self.LoadingScreenTexture`) (`self.MapNameText`)))

(fn `UserConstructionScript`)