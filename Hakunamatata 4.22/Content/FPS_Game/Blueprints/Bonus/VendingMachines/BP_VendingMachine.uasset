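; BP_VendingMachine is an interactable vending machine that opens a shop-style UI when used.
; Overlap begin and end events cast to BP_CharacterBase and show or hide the interact prompt text on that character's HUD.
; The interaction interface event creates a W_VendingMachineUI widget and adds it to the viewport.
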(event `self.ReceiveActorBeginOverlap`
  (params (OtherActor :type "Actor Object Reference"))
  (bind _asbp_character_base (cast `/Game/ThirdPersonBP/BP_CharacterBase` OtherActor))
  (`Widget.SetVisibility` (`/Game/FPS_Game/UI/W_PlayerHUD.InteractPrompt_TXT` (`/Game/ThirdPersonBP/BP_CharacterBase.PlayerHUD` _asbp_character_base)) "Visible"))

(event `self.ReceiveActorEndOverlap`
  (params (OtherActor :type "Actor Object Reference"))
  (bind _asbp_character_base (cast `/Game/ThirdPersonBP/BP_CharacterBase` OtherActor))
  (`Widget.SetVisibility` (`/Game/FPS_Game/UI/W_PlayerHUD.InteractPrompt_TXT` (`/Game/ThirdPersonBP/BP_CharacterBase.PlayerHUD` _asbp_character_base)) "Hidden"))

(event `/Game/FPS_Game/Blueprints/System/BPI_Interact.BPI_Interaction`
  (bind _returnvalue (`|CreateWidget` "/Game/FPS_Game/UI/W_VendingMachineUI.W_VendingMachineUI_C"))
  (`UserWidget.AddToViewport` _returnvalue 0))

(fn `UserConstructionScript`)