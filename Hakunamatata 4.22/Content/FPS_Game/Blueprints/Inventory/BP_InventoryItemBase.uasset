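; Base actor for inventory pickups that the Joe player character can store in a universal inventory.
; On BeginPlay it builds its item data struct and, for non-respawning classes, hides itself after a short delay if the inventory holds that class.
; Sphere overlap toggles custom depth highlighting and Visibility trace blocking.
; StoreThisItem adds the item, hiding it and disabling sphere collision, or prints a message when full.
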(event `self.ReceiveBeginPlay`
  (bind _asjoe (cast `/Game/ThirdPersonBP/Joe` (`GameplayStatics.GetPlayerCharacter` 0)))
  (set `self.PlayerCast` _asjoe)
  (bind _output_get (set `self.ThisItem` self))
  (set `self.IntentoryDataStruct` (make `/Game/FPS_Game/Blueprints/Inventory/S_InventoryItemStruct` _output_get (`GameplayStatics.GetObjectClass` self) (`self.ItemName`) (`self.ItemImage`)))
  (`KismetSystemLibrary.Delay` 0.2)
  (if (not (`self.ClassCanRespawn`))
    (for _array_element (`/Game/ThirdPersonBP/Joe.Universal_Inventory` (`self.PlayerCast`))
      (if (== (`GameplayStatics.GetObjectClass` _array_element) (`GameplayStatics.GetObjectClass` self))
        (`self.SetActorHiddenInGame` true)
        (`PrimitiveComponent.SetCollisionEnabled` (`self.Sphere`) "NoCollision")))))

(event `self.Sphere.OnComponentBeginOverlap`
  (params (OverlappedComponent :type "PrimitiveComponent Object Reference") (OtherActor :type "Actor Object Reference") (OtherComp :type "PrimitiveComponent Object Reference") (OtherBodyIndex :type Integer) (bFromSweep :type Boolean) (SweepResult :type "HitResult Structure (by ref)"))
  (cast `/Game/ThirdPersonBP/Joe` OtherActor)
  (`PrimitiveComponent.SetRenderCustomDepth` (`self.Mesh`) true)
  (`PrimitiveComponent.SetCollisionResponseToChannel` (`self.Sphere`) "ECC_Visibility" "ECR_Block"))

(event `self.Sphere.OnComponentEndOverlap`
  (params (OverlappedComponent :type "PrimitiveComponent Object Reference") (OtherActor :type "Actor Object Reference") (OtherComp :type "PrimitiveComponent Object Reference") (OtherBodyIndex :type Integer))
  (cast `/Game/ThirdPersonBP/Joe` OtherActor)
  (`PrimitiveComponent.SetRenderCustomDepth` (`self.Mesh`) false)
  (`PrimitiveComponent.SetCollisionResponseToChannel` (`self.Sphere`) "ECC_Visibility" "ECR_Ignore"))

(fn `StoreThisItem`
  (bind _playercast (`self.PlayerCast`))
  (if (< (`KismetArrayLibrary.Array_Length` (`/Game/ThirdPersonBP/Joe.Universal_Inventory` _playercast)) (`/Game/ThirdPersonBP/Joe.UniversalItemLimit` _playercast))
    (`/Game/ThirdPersonBP/Joe.AddItemToUniversalInventory` (`self.PlayerCast`) (`self.ThisItem`))
    (`PrimitiveComponent.SetCollisionEnabled` (`self.Sphere`) "NoCollision")
    (`self.SetActorHiddenInGame` true)
    (else
      (`KismetSystemLibrary.PrintString` "Universal Item Inventory Full"))))

(fn `UserConstructionScript`)