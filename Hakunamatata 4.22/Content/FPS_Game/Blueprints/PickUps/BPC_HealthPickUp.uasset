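; Health pickup Blueprint that either heals the player or is stored as an item.
; Use and interaction events compare current health to max: below max it heals by HealthToAdd and destroys itself, otherwise it calls StoreThisItem.
; Overlap with a Joe below max health triggers the same heal-and-destroy path through the PlayerCast reference, and never stores the item.
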(event `/Game/FPS_Game/Blueprints/Inventory/BPI_ItemInterface.BPI_UseItem`
  (bind _playercast (`self.PlayerCast`))
  (`/Engine/EditorBlueprintResources/StandardMacros.CompareFloat` (`/Game/ThirdPersonBP/Joe.HealthCurrent` _playercast) (`/Game/ThirdPersonBP/Joe.HealthMax` _playercast) :!label _label
    (:`>`
      (`self.StoreThisItem` :!label _label_2))
    (:`==`
      (goto _label_2))
    (:`<`
      (`/Game/ThirdPersonBP/Joe.HealthHeal` (`self.PlayerCast`) (`self.HealthToAdd`) :!label _label_3)
      (`self.K2_DestroyActor`))))

(event `/Game/FPS_Game/Blueprints/System/BPI_Interact.BPI_Interaction`
  (goto _label))

(event `self.ReceiveActorBeginOverlap`
  (params (OtherActor :type "Actor Object Reference"))
  (bind _asjoe (cast `/Game/ThirdPersonBP/Joe` OtherActor))
  (if (< (`/Game/ThirdPersonBP/Joe.HealthCurrent` _asjoe) (`/Game/ThirdPersonBP/Joe.HealthMax` _asjoe))
    (goto _label_3)))

(fn `UserConstructionScript`
  (`parent.UserConstructionScript`))