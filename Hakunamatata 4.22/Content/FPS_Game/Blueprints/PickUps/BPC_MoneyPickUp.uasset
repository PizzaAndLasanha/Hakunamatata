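; Money pickup Blueprint that spins continuously in the world.
; Each Tick subtracts RotationSpeed from the DefaultSceneRoot's world yaw, keeping roll and pitch, with no delta-time scaling.
; BeginPlay and the construction script only call the parent, and the Tick parent call is disabled.
; The overlap event is a disabled stub, so this graph holds no collection or money logic.
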(event `self.ReceiveTick`
  (params (DeltaSeconds :type "Float (single-precision)"))
  (bind (_returnvalue_roll _returnvalue_pitch _returnvalue_yaw) (`KismetMathLibrary.BreakRotator` (`SceneComponent.K2_GetComponentRotation` (`self.DefaultSceneRoot`))))
  (`SceneComponent.K2_SetWorldRotation` (`self.DefaultSceneRoot`) (`KismetMathLibrary.MakeRotator` _returnvalue_roll _returnvalue_pitch (- _returnvalue_yaw (`self.RotationSpeed`))) false false))

(event `self.ReceiveBeginPlay`
  (`parent.ReceiveBeginPlay`))

(fn `UserConstructionScript`
  (`parent.UserConstructionScript`))