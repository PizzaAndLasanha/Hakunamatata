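; Animated NPC Blueprint for the dialogue system, scripted with a placeholder test conversation.
; After conversation setup it adds an important dialogue line under the NPC's name.
; When dialogue ends, an index switch adds a three-option decision, and the decision-made handler switches on the choice and ends the conversation.
; BeginPlay and construction only call the parent class, and no animation logic appears in these graphs.
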(event `self.AfterConversationSetup`
  (`self.AddCustomImportantDialogue` 0 (make `/Game/DialogueSystem/Blueprints/Structures/s_DialogueInfo` null "this is working" (`self.Name`))))

(event `self.OnDialogueEnd`
  (params (Index :type Integer))
  (switch `int` Index
    (:`Default`
      (`self.AddDecision` 0 (make `/Game/DialogueSystem/Blueprints/Structures/s_DecisionInfo` (make `/Game/DialogueSystem/Blueprints/Structures/s_DialogueInfo` null "choose options now") (`|MakeArray` (make `/Game/DialogueSystem/Blueprints/Structures/s_OptionInfo` "option 1") (make `/Game/DialogueSystem/Blueprints/Structures/s_OptionInfo` "option 2") (make `/Game/DialogueSystem/Blueprints/Structures/s_OptionInfo` "option 3") :!type "/Game/DialogueSystem/Blueprints/Structures/s_OptionInfo Structure"))))))

(event `self.OnDecisionMade`
  (params (DecisionIndex :type Integer) (ChosenOptionIndex :type Integer))
  (switch `int` DecisionIndex
    (:`Default`
      (`self.EndConversation`))))

(event `self.ReceiveBeginPlay`
  (`parent.ReceiveBeginPlay`))

(fn `UserConstructionScript`
  (`parent.UserConstructionScript`))