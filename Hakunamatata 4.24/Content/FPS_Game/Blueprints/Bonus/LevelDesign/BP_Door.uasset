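; BP_Door is a sliding double door that opens automatically when a character derived from BP_CharacterBase enters its trigger box.
; Box overlap begin plays the Door_TL timeline and overlap end reverses it.
; The timeline's alpha lerps the left and right panels between their closed and open relative locations.
; Exits are not counted, so any character leaving starts closing the door even if another remains inside.
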(event `self.Box.OnComponentBeginOverlap`
  (params (OverlappedComponent :type "PrimitiveComponent Object Reference") (OtherActor :type "Actor Object Reference") (OtherComp :type "PrimitiveComponent Object Reference") (OtherBodyIndex :type Integer) (bFromSweep :type Boolean) (SweepResult :type "HitResult Structure (by ref)"))
  (cast `/Game/ThirdPersonBP/BP_CharacterBase` OtherActor)
  (bind (_direction _alpha) (`Timeline|Door_TL` :!label _label)
    (:`Update`
      (`SceneComponent.K2_SetRelativeLocation` (`self.Door_L`) (`KismetMathLibrary.VLerp` (`self.Door_L_Closed`) (`self.Door_L_Open`) _alpha) false false)
      (`SceneComponent.K2_SetRelativeLocation` (`self.Door_R`) (`KismetMathLibrary.VLerp` (`self.Door_R_Closed`) (`self.Door_R_Open`) _alpha) false false))))

(event `self.Box.OnComponentEndOverlap`
  (params (OverlappedComponent :type "PrimitiveComponent Object Reference") (OtherActor :type "Actor Object Reference") (OtherComp :type "PrimitiveComponent Object Reference") (OtherBodyIndex :type Integer))
  (cast `/Game/ThirdPersonBP/BP_CharacterBase` OtherActor)
  (goto _label :!via `Reverse`))

(fn `UserConstructionScript`)