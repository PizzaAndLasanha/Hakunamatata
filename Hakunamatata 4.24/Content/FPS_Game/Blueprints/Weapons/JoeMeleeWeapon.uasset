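; Joe's melee weapon Blueprint, where both fire and aim-down-sights inputs trigger one slashing attack.
; MeleeWeapon plays first-person and randomized third-person montages, then after a delay line-traces by view mode: via the player in first person, from the capsule otherwise.
; Hits apply point damage, sparks and sound, with IsMeleeAttacking blocking overlapping swings.
; Head hits double DamageVar, which is copied into Damage only after damage is applied.
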(event `self.ReceiveBeginPlay`
  (`parent.ReceiveBeginPlay`))

(event `self.ADS_Override`
  (bind _playercast (`self.PlayerCast`))
  (bind _capsulecomponent (`Character.CapsuleComponent` _playercast))
  (bind _returnvalue (`SceneComponent.K2_GetComponentLocation` _capsulecomponent))
  (if (not (`self.isMeleeAttacking`)) :!label _label
    (set `self.isMeleeAttacking` true)
    (`|ExecutionSequence`
      (:`then_0`
        (bind _returnvalue_2 (`AnimInstance.Montage_Play` (`SkeletalMeshComponent.GetAnimInstance` (`/Game/ThirdPersonBP/BP_CharacterBase.Mesh_FPP` _playercast)) (`self.MeleeMontage1`) 2.0 "Duration" 0.0 true))
        (`KismetSystemLibrary.Delay` (/ _returnvalue_2 1.5))
        (if (`/Game/ThirdPersonBP/BP_CharacterBase.isFPP` _playercast)
          (bind (_returnvalue_3 _outhit) (`/Game/ThirdPersonBP/BP_CharacterBase.LinetraceByChannel` _playercast 300.0 0.0 "None"))
          (if _returnvalue_3
            (bind (_bblockinghit _binitialoverlap _time _distance _location _impactpoint _normal _impactnormal _physmat _hitactor _hitcomponent _hitbonename) (`GameplayStatics.BreakHitResult` _outhit))
            (`self.CriticalHitCheck` _hitbonename)
            (`GameplayStatics.ApplyPointDamage` _hitactor (`self.Damage`) _location (`GameplayStatics.MakeHitResult` (`GameplayStatics.BreakHitResult` (stale `self.ReceiveHit` Hit)) (`.bInitialOverlap` (`GameplayStatics.BreakHitResult` (stale `self.ReceiveHit` Hit))) (`.Time` (`GameplayStatics.BreakHitResult` (stale `self.ReceiveHit` Hit))) 0.0 (`.Location` (`GameplayStatics.BreakHitResult` (stale `self.ReceiveHit` Hit))) (`.ImpactPoint` (`GameplayStatics.BreakHitResult` (stale `self.ReceiveHit` Hit))) (`.Normal` (`GameplayStatics.BreakHitResult` (stale `self.ReceiveHit` Hit))) (`.ImpactNormal` (`GameplayStatics.BreakHitResult` (stale `self.ReceiveHit` Hit))) (`.PhysMat` (`GameplayStatics.BreakHitResult` (stale `self.ReceiveHit` Hit))) (`.HitActor` (`GameplayStatics.BreakHitResult` (stale `self.ReceiveHit` Hit))) (`.HitComponent` (`GameplayStatics.BreakHitResult` (stale `self.ReceiveHit` Hit))) (`.HitBoneName` (`GameplayStatics.BreakHitResult` (stale `self.ReceiveHit` Hit))) (`.HitItem` (`GameplayStatics.BreakHitResult` (stale `self.ReceiveHit` Hit))) (`.FaceIndex` (`GameplayStatics.BreakHitResult` (stale `self.ReceiveHit` Hit))) (`.TraceStart` (`GameplayStatics.BreakHitResult` (stale `self.ReceiveHit` Hit))) (`.TraceEnd` (`GameplayStatics.BreakHitResult` (stale `self.ReceiveHit` Hit)))) null null "/Game/LitoStudy/AttackTypes/AttackTypes_Slash.AttackTypes_Slash_C" :!label _label_2)
            (set `self.Damage` (`self.DamageVar`))
            (`GameplayStatics.SpawnEmitterAtLocation` "/Game/FPS_Game/Weapons/Effects/ParticleSystems/Weapons/AssaultRifle/Impacts/P_AssaultRifle_IH_SparksOnly.P_AssaultRifle_IH_SparksOnly" _location (`KismetMathLibrary.RandomRotator` false))
            (`GameplayStatics.PlaySoundAtLocation` "/Game/FPS_Game/Sounds/SFX/CharacterRelated/FightMatinee/Impact_Punch_Harder_Cue.Impact_Punch_Harder_Cue" (`self.K2_GetActorLocation`) (struct) 1.0 1.0 0.0 null null null))
          (else
            (bind (_outhit_2 _returnvalue_4) (`KismetSystemLibrary.LineTraceSingle` (+ _returnvalue (0.0 0.0 50.0)) (+ (* (`SceneComponent.GetForwardVector` _capsulecomponent) 120.0) _returnvalue) "TraceTypeQuery1" false (`self.ActorsToIgnore`)))
            (if _returnvalue_4
              (bind (_bblockinghit_2 _binitialoverlap_2 _time_2 _distance_2 _location_2 _impactpoint_2 _normal_2 _impactnormal_2 _physmat_2 _hitactor_2 _hitcomponent_2 _hitbonename_2) (`GameplayStatics.BreakHitResult` _outhit_2))
              (`self.CriticalHitCheck` _hitbonename_2)
              (`GameplayStatics.ApplyPointDamage` _hitactor_2 (`self.Damage`) _location_2 _outhit_2 null null "/Game/LitoStudy/AttackTypes/AttackTypes_Slash.AttackTypes_Slash_C")
              (set `self.Damage` (`self.DamageVar`))
              (`GameplayStatics.SpawnEmitterAtLocation` "/Game/FPS_Game/Weapons/Effects/ParticleSystems/Weapons/AssaultRifle/Impacts/P_AssaultRifle_IH_SparksOnly.P_AssaultRifle_IH_SparksOnly" _location_2 (`KismetMathLibrary.RandomRotator` false))
              (`GameplayStatics.PlaySoundAtLocation` "/Game/FPS_Game/Sounds/SFX/CharacterRelated/FightMatinee/Impact_Punch_Harder_Cue.Impact_Punch_Harder_Cue" (`self.K2_GetActorLocation`) (struct) 1.0 1.0 0.0 null null null))))
        (set `self.isMeleeAttacking` false))
      (:`then_1`
        (`AnimInstance.Montage_Play` (`SkeletalMeshComponent.GetAnimInstance` (`Character.Mesh` _playercast)) (select `bool` (`KismetMathLibrary.RandomBool`) :`false` (`self.TPS_MeleeMontage1`) :`true` (`self.TPS_MeleeMontage2`)) 1.5 "Duration" 0.0 true)))))

(event `self.WeaponFire`
  (goto _label))

(event `self.ReceiveHit`
  (params (MyComp :type "PrimitiveComponent Object Reference") (Other :type "Actor Object Reference") (OtherComp :type "PrimitiveComponent Object Reference") (bSelfMoved :type Boolean) (HitLocation :type "Vector Structure") (HitNormal :type "Vector Structure") (NormalImpulse :type "Vector Structure") (Hit :type "HitResult Structure (by ref)"))
  (goto _label_2))

(fn `UserConstructionScript`
  (`parent.UserConstructionScript`))