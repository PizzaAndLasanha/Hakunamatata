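; Key pickup that gives the player character a key on touch, built on a universal item pickup template.
; Overlap with a BP_CharacterBase adds a fixed single key, prints a message using KeyToAdd, then destroys the sphere and actor.
; The interaction event is empty, the use-item event keeps the template's placeholder print and destroy, and an unconnected branch would add a key and store the item.
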(event `/Game/FPS_Game/Blueprints/System/BPI_Interact.BPI_Interaction`
  ;[1 1 1] Blank example for an universal item pickup, duplicate it and replace the ITEM USED Print String with whatever logic you need it to do.
)

(event `/Game/FPS_Game/Blueprints/Inventory/BPI_ItemInterface.BPI_UseItem`
  ;[1 1 1] Blank example for an universal item pickup, duplicate it and replace the ITEM USED Print String with whatever logic you need it to do.
  (`KismetSystemLibrary.PrintString` "ITEM USED") ; Your item logic goes here
  (`self.K2_DestroyActor`))

(event `self.ReceiveActorBeginOverlap`
  (params (OtherActor :type "Actor Object Reference"))
  (bind _asbp_character_base (cast `/Game/ThirdPersonBP/BP_CharacterBase` OtherActor))
  (`/Game/ThirdPersonBP/BP_CharacterBase.AddKeys` _asbp_character_base 1)
  (`KismetSystemLibrary.PrintString` (`KismetStringLibrary.Concat_StrStr` (`KismetStringLibrary.Conv_IntToString` (`self.KeyToAdd`)) "Key"))
  (`ActorComponent.K2_DestroyComponent` (`self.Sphere`))
  (`self.K2_DestroyActor`))

(fn `UserConstructionScript`
  (`parent.UserConstructionScript`))