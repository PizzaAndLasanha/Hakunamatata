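; Money pickup Blueprint that spins its Cube as a visual effect; it contains no collection or currency logic of its own.
; Each Tick subtracts RotationSpeed from the Cube's world yaw, keeping roll and pitch, so the spin rate depends on frame rate.
; BeginPlay and the construction script only call the parent, and the overlap event is disabled.
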(event `self.ReceiveTick`
  (params (DeltaSeconds :type "Float (single-precision)"))
  (bind _cube (`self.Cube`))
  (bind (_returnvalue_roll _returnvalue_pitch _returnvalue_yaw) (`KismetMathLibrary.BreakRotator` (`SceneComponent.K2_GetComponentRotation` _cube)))
  (`SceneComponent.K2_SetWorldRotation` _cube (`KismetMathLibrary.MakeRotator` _returnvalue_roll _returnvalue_pitch (- _returnvalue_yaw (`self.RotationSpeed`))) false false))

(event `self.ReceiveBeginPlay`
  (`parent.ReceiveBeginPlay`))

(fn `UserConstructionScript`
  (`parent.UserConstructionScript`))