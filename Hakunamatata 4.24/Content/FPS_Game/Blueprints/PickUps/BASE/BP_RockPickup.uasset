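; Rock pickup actor that adds one rock to the player character's supply when interacted with.
; On BeginPlay it caches player 0 as BP_CharacterBase, and its BPIInteraction event compares that character's CurrentRocks to MaxRocks.
; Below the limit it calls AddRocks and destroys itself; otherwise it stays in the world.
; Both outcomes print debug messages that refer to grenades rather than rocks.
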(event `self.ReceiveBeginPlay`
  (bind _asbp_character_base (cast `/Game/ThirdPersonBP/BP_CharacterBase` (`GameplayStatics.GetPlayerCharacter` 0)))
  (set `self.PlayerCast` _asbp_character_base))

(event `/Game/FPS_Game/Blueprints/System/BPI_Interact.BPI_Interaction`
  (bind _playercast (`self.PlayerCast`))
  (`/Engine/EditorBlueprintResources/StandardMacros.CompareInt` (`/Game/ThirdPersonBP/BP_CharacterBase.CurrentRocks` _playercast) (`/Game/ThirdPersonBP/BP_CharacterBase.MaxRocks` _playercast)
    (:`>`
      (`KismetSystemLibrary.PrintString` "MAX  GRENADES" :!label _label))
    (:`==`
      (goto _label))
    (:`<`
      (`/Game/ThirdPersonBP/BP_CharacterBase.AddRocks` _playercast 1)
      (`KismetSystemLibrary.PrintString` "GRENADE  ADDED")
      (`self.K2_DestroyActor`))))

(fn `UserConstructionScript`)