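; BP_FPPT_Bridge is a powered interactable bridge that extends from a Start piece toward an End piece at EndPosition.
; Inherited power update and finish events drive UpdatePositions, which orients both end pieces along the span and stretches the Bridge mesh by moving its midpoint and scaling its length.
; The construction script sizes the end pieces from Width, and SetupMaterialOwners gives all three meshes the main power material.
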(event `self.ReceiveBeginPlay`
  (`parent.ReceiveBeginPlay`))

(event `self.Setup Material Owners`
  (`PrimitiveComponent.SetMaterial` (`self.Start`) 0 (`self.Main Power Material`))
  (`PrimitiveComponent.SetMaterial` (`self.Bridge`) 0 (`self.Main Power Material`))
  (`PrimitiveComponent.SetMaterial` (`self.End`) 0 (`self.Main Power Material`)))

(event `self.On Update Power Update`
  (params (`Current Amount` :type "Float (single-precision)"))
  (`self.UpdatePositions` `Current Amount`))

(event `self.On Update Power Finished`
  (params (Forced :type Boolean))
  (`self.UpdatePositions` (`KismetMathLibrary.Conv_BoolToDouble` (`self.Active`))))

(fn `UpdatePositions`
  (params (Amount :type "Float (double-precision)"))
  (bind _returnvalue (`KismetMathLibrary.MakeVector` 0.0))
  (bind _end_position (`self.End Position`))
  (bind _returnvalue_2 (`KismetMathLibrary.FindLookAtRotation` _end_position _returnvalue))
  (bind _returnvalue_3 (`KismetMathLibrary.VLerp` (0.0 0.0 0.0) (`self.End Position`) (`local.Amount`)))
  (`SceneComponent.K2_SetRelativeRotation` (`self.Start`) (`KismetMathLibrary.TransformRotation` (`KismetMathLibrary.MakeTransform` (0.0 0.0 0.0) _returnvalue_2) (struct :`Yaw` 90.0)) false false)
  (`SceneComponent.K2_SetRelativeLocationAndRotation` (`self.End`) (`self.End Position`) (`KismetMathLibrary.TransformRotation` (`KismetMathLibrary.MakeTransform` (0.0 0.0 0.0) (`KismetMathLibrary.FindLookAtRotation` _returnvalue _end_position)) (struct :`Yaw` 90.0)) false false)
  (`SceneComponent.K2_SetRelativeLocationAndRotation` (`self.Bridge`) (+ (/ (0.0 0.0 0.0) 2.0) (/ _returnvalue_3 2.0)) _returnvalue_2 false false)
  (`SceneComponent.SetRelativeScale3D` (`self.Bridge`) (`KismetMathLibrary.MakeVector` (`KismetMathLibrary.FMax` (/ (`KismetMathLibrary.VSize` (- (0.0 0.0 0.0) _returnvalue_3)) 100.0) 0.01) (* (`self.Width`) 1.35) 0.35)))

(fn `UserConstructionScript`
  (`parent.UserConstructionScript`)
  (`SceneComponent.SetRelativeScale3D` (`self.Start`) (`KismetMathLibrary.MakeVector` (`self.Width`) 1.0 1.0))
  (`SceneComponent.SetRelativeScale3D` (`self.End`) (`KismetMathLibrary.MakeVector` (`self.Width`) 1.0 1.0)))