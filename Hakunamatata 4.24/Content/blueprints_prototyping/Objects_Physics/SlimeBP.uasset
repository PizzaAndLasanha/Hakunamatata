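; Physics prototype slime actor that acts as a ball the player can kick with the left mouse button.
; Box collision overlap enables input on the actor and end overlap disables it, without checking which actor overlaps or where it faces.
; A click applies a velocity-change impulse to BallMesh along the player controller's forward vector, scaled by Kickspeed, and prints a debug message.
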(event `self.ReceiveBeginPlay`)

(event `self.ReceiveTick`
  (params (DeltaSeconds :type "Float (single-precision)")))

(event `Key|LeftMouseButton`
  (params (Key :type "Key Structure"))
  ;[1 1 1] when ball is kicked give it an impulse in the direction the player is facing
  (:`Pressed`
    (`PrimitiveComponent.AddImpulse` (`self.ball_mesh`) (* (`self.GetActorForwardVector` (`GameplayStatics.GetPlayerController` 0)) (`self.Kickspeed`)) "None" true)
    (`KismetSystemLibrary.PrintString` "Ball kicked")))

(event `self.Boxcollision.OnComponentBeginOverlap`
  (params (OverlappedComponent :type "PrimitiveComponent Object Reference") (OtherActor :type "Actor Object Reference") (OtherComp :type "PrimitiveComponent Object Reference") (OtherBodyIndex :type Integer) (bFromSweep :type Boolean) (SweepResult :type "HitResult Structure (by ref)"))
  ;[1 1 1] Enables or disables input when we are inside collision (it still works if we are facing back for now)
  (`self.EnableInput` (`GameplayStatics.GetPlayerController` 0)))

(event `self.Boxcollision.OnComponentEndOverlap`
  (params (OverlappedComponent :type "PrimitiveComponent Object Reference") (OtherActor :type "Actor Object Reference") (OtherComp :type "PrimitiveComponent Object Reference") (OtherBodyIndex :type Integer))
  ;[1 1 1] Enables or disables input when we are inside collision (it still works if we are facing back for now)
  (`self.DisableInput` (`GameplayStatics.GetPlayerController` 0)))

(fn `UserConstructionScript`)