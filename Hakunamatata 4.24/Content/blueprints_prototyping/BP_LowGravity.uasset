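; Prototype low-gravity volume actor that makes characters float while they overlap it.
; On BeginPlay it caches the player character's movement gravity scale as the default.
; Any BP_CharacterBase entering the overlap gets a much lower GravityScale, and on exit receives that cached player default rather than its own original value.
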(event `self.ReceiveBeginPlay`
  (set `self.DefaultGtavity` (`CharacterMovementComponent.GravityScale` (`Character.CharacterMovement` (`/Game/FPS_Game/Blueprints/System/BP_Library.GetPlayerCast`)))))

(event `self.ReceiveActorBeginOverlap`
  (params (OtherActor :type "Actor Object Reference"))
  (bind _asbp_character_base (cast `/Game/FPS_Game/Blueprints/BP_CharacterBase` OtherActor))
  (set `CharacterMovementComponent.GravityScale` 0.1 (`Character.CharacterMovement` _asbp_character_base)))

(event `self.ReceiveActorEndOverlap`
  (params (OtherActor :type "Actor Object Reference"))
  (bind _asbp_character_base (cast `/Game/FPS_Game/Blueprints/BP_CharacterBase` OtherActor))
  (set `CharacterMovementComponent.GravityScale` (`self.DefaultGtavity`) (`Character.CharacterMovement` _asbp_character_base)))

(fn `UserConstructionScript`)