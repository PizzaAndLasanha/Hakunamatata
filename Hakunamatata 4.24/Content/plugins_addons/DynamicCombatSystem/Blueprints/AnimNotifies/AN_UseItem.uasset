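; Anim notify in the Dynamic Combat System that uses an item from the owner's equipment at a specific point in an animation.
; It looks up the mesh owner's equipment and inventory components, gets the active item in the first slot of the configured Type, and passes its ID to the inventory's UseItem.
; The notify's name is built from that Type.
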(fn `GetNotifyName`
  (returns (ReturnValue :type String))
  (return (`KismetStringLibrary.Concat_StrStr` "Use " (`|GetEnumeratorNameAsString` (`self.Type`)))))

(fn `Received_Notify`
  (params (MeshComp :type "SkeletalMeshComponent Object Reference") (Animation :type "AnimSequenceBase Object Reference"))
  (returns (ReturnValue :type Boolean))
  (locals (L_Equipment :type "/Game/plugins_addons/DynamicCombatSystem/Blueprints/Components/EquipmentComponent Object Reference") (L_Inventory :type "/Game/plugins_addons/DynamicCombatSystem/Blueprints/Components/InventoryComponent Object Reference"))
  (bind _returnvalue (`ActorComponent.GetOwner` MeshComp))
  (`/Engine/EditorBlueprintResources/StandardMacros.IsValid` _returnvalue
    (:`Is Valid`
      (set `local.L_Equipment` (`Actor.GetComponentByClass` _returnvalue "/Game/plugins_addons/DynamicCombatSystem/Blueprints/Components/EquipmentComponent.EquipmentComponent_C"))
      (set `local.L_Inventory` (`Actor.GetComponentByClass` _returnvalue "/Game/plugins_addons/DynamicCombatSystem/Blueprints/Components/InventoryComponent.InventoryComponent_C"))
      (bind _l_equipment (`local.L_Equipment`)
        (:`then`
          (bind _l_inventory (`local.L_Inventory`)
            (:`then`
              (`/Game/plugins_addons/DynamicCombatSystem/Blueprints/Components/InventoryComponent.UseItem` _l_inventory (`.Id_14_053D433B49C6A6BD4B72C8A74C0D15E1` (break `/Game/plugins_addons/DynamicCombatSystem/Structs/F_StoredItem` (`/Game/plugins_addons/DynamicCombatSystem/Blueprints/Components/EquipmentComponent.GetActiveItem` _l_equipment (`self.Type`) 0))))
              (return false))
            (:`else`)))
        (:`else`)))))