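; BP_BaseModuleWeapon is a base Blueprint for trap weapon modules in the DeathTraps pack, holding shared damage and impulse settings.
; SetNewDamage overwrites the damage, impulse and custom-impulse flag.
; CauseDamage messages targets implementing BPI_CustomDamage with the damage and either the custom impulse or the passed mesh's physics linear velocity.
; Its event graph and construction script are empty, so it triggers no damage itself.
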(fn `CauseDamage`
  (params (Player :type "Actor Object Reference") (Mesh :type "PrimitiveComponent Object Reference"))
  ;[1 1 1] Check actor for interface
  (if (`KismetSystemLibrary.DoesImplementInterface` Player "/Game/plugins_addons/DeathTrapsVol_1/Blueprints/Interfaces/BPI_CustomDamage.BPI_CustomDamage_C")
    (bind _returnvalue (`PrimitiveComponent.GetPhysicsLinearVelocity` Mesh "None")) ; Get velocity mesh for add character impulse
    (message `/Game/plugins_addons/DeathTrapsVol_1/Blueprints/Interfaces/BPI_CustomDamage.ApplyCustomDamage` Player (`self.Damage`) (select `bool` (`self.bCustomImpulse`) :`false` _returnvalue :`true` (`self.Impulse`)) 0 "None" null)))

(fn `SetNewDamage`
  (params (NewDamage :type "Float (double-precision)") (Impulse :type "Vector Structure") (bCustomImpulse :type Boolean))
  ;[1 1 1] Set new settings
  (set `self.Damage` NewDamage)
  (set `self.Impulse` Impulse)
  (set `self.bCustomImpulse` bCustomImpulse))

(fn `UserConstructionScript`)