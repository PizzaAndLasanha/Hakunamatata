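; BP_SpikeLogRotation is a rotating spike log trap Blueprint built on a parent trap class.
; Its construction script assigns the WeaponClass to a child actor component and sets that component's starting rotation from the DirectionAnimation setting, using the end rotation for backward motion and the start rotation otherwise.
; BeginPlay and Tick only forward to the parent, which handles any runtime behavior.
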(event `self.ReceiveBeginPlay`
  (`parent.ReceiveBeginPlay`))

(event `self.ReceiveTick`
  (params (DeltaSeconds :type "Float (single-precision)"))
  (`parent.ReceiveTick` DeltaSeconds))

(fn `UserConstructionScript`
  (bind _rotationstart (`self.RotationStart`))
  (`parent.UserConstructionScript`)
  (`ChildActorComponent.SetChildActorClass` (`self.BP_ChildActor`) (`self.WeaponClass`)) ; Set weapon class
  ;[1 1 1] Start rotation trap by direction animation
  (`SceneComponent.K2_SetRelativeRotation` (`self.BP_ChildActor`) (select `/Game/plugins_addons/DeathTrapsVol_1/Blueprints/Enumeration/E_DirectionsAnimation` (`self.DirectionAnimation`) :`NewEnumerator0` _rotationstart :`NewEnumerator1` _rotationstart :`NewEnumerator2` (`self.RotationEnd`)) false false))