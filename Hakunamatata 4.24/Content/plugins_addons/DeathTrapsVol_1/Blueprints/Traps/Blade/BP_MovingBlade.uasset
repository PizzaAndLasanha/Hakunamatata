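; BP_MovingBlade is a trap Blueprint that slides a child-actor blade weapon between a start and end location.
; On BeginPlay it passes damage, impulse and custom impulse to the BP_BaseModuleWeapon inside the child actor.
; The AnimationLogic event lerps the blade's relative X and Y independently, using FrameAnimation's Y component for X and its X component for Y.
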(event `self.ReceiveBeginPlay`
  (`parent.ReceiveBeginPlay`)
  ;[1 1 1] Set new damage settings
  (`/Engine/EditorBlueprintResources/StandardMacros.IsValid` (`self.BP_ChildActor`)
    (:`Is Valid`
      (bind _asbp_base_module_weapon (cast `/Game/plugins_addons/DeathTrapsVol_1/Blueprints/Traps/BP_BaseModuleWeapon` (`ChildActorComponent.ChildActor` (`self.BP_ChildActor`))))
      (`/Game/plugins_addons/DeathTrapsVol_1/Blueprints/Traps/Blade/BP_Blade_01.SetNewDamage` _asbp_base_module_weapon (`self.Damage`) (`self.Impulse`) (`self.bCustomImpulse`)))))

(event `self.AnimationLogic`
  (bind (_frameanimation_x _frameanimation_y) (`KismetMathLibrary.BreakVector` (`self.FrameAnimation`)))
  (bind (_locationstart_x _locationstart_y) (`KismetMathLibrary.BreakVector` (`self.LocationStart`)))
  (bind (_locationend_x _locationend_y) (`KismetMathLibrary.BreakVector` (`self.LocationEnd`)))
  (`SceneComponent.K2_SetRelativeLocation` (`self.BP_ChildActor`) (`KismetMathLibrary.MakeVector` (`KismetMathLibrary.Lerp` _locationstart_x _locationend_x _frameanimation_y) (`KismetMathLibrary.Lerp` _locationstart_y _locationend_y _frameanimation_x)) false false))

(fn `UserConstructionScript`
  (`parent.UserConstructionScript`))