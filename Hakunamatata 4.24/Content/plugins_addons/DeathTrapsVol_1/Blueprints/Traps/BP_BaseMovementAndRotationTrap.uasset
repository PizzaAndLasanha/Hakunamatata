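; Base trap Blueprint that moves and rotates a child-actor weapon between configurable start and end transforms.
; Construction sets the weapon class and initial transform from the animation direction.
; BeginPlay passes damage and impulse to the weapon, swapping start and end values for Backward.
; AnimationLogic lerps rotation by FrameAnimation.X and location by Y, with rotation's endpoints ordered end-to-start, opposite to location's.
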(event `self.ReceiveBeginPlay`
  (`parent.ReceiveBeginPlay`)
  (`|ExecutionSequence`
    (:`then_0`
      ;[1 1 1] Set new damage settings
      (`/Engine/EditorBlueprintResources/StandardMacros.IsValid` (`self.BP_ChildActor`)
        (:`Is Valid`
          (bind _asbp_base_module_weapon (cast `/Game/plugins_addons/DeathTrapsVol_1/Blueprints/Traps/BP_BaseModuleWeapon` (`ChildActorComponent.ChildActor` (`self.BP_ChildActor`))))
          (`/Game/plugins_addons/DeathTrapsVol_1/Blueprints/Traps/BP_BaseModuleWeapon.SetNewDamage` _asbp_base_module_weapon (`self.Damage`) (`self.Impulse`) (`self.bCustomImpulse`)))))
    (:`then_1`
      ;[1 1 1] Swap variables
      (switch `/Game/plugins_addons/DeathTrapsVol_1/Blueprints/Enumeration/E_DirectionsAnimation` (`self.DirectionAnimation`)
        (:`NewEnumerator2`
          (set `self.TempRotationStart` (`self.RotationStart`))
          (set `self.RotationStart` (`self.RotationEnd`))
          (set `self.RotationEnd` (`self.TempRotationStart`))
          (set `self.TempLocationStart` (`self.LocationStart`))
          (set `self.LocationStart` (`self.LocationEnd`))
          (set `self.LocationEnd` (`self.TempLocationStart`)))))))

(event `self.AnimationLogic`
  (bind _frameanimation_x (`KismetMathLibrary.BreakVector` (`self.FrameAnimation`)))
  (bind (_frameanimation_x_2 _frameanimation_y) (`KismetMathLibrary.BreakVector` (`self.FrameAnimation`)))
  ;[1 1 1] Logic rotation and location animation
  (`SceneComponent.K2_SetRelativeRotation` (`self.BP_ChildActor`) (`KismetMathLibrary.RLerp` (`self.RotationEnd`) (`self.RotationStart`) _frameanimation_x) false false)
  (`SceneComponent.K2_SetRelativeLocation` (`self.BP_ChildActor`) (`KismetMathLibrary.VLerp` (`self.LocationStart`) (`self.LocationEnd`) _frameanimation_y) false false))

(fn `UserConstructionScript`
  (bind _rotationstart (`self.RotationStart`))
  (bind _locationstart (`self.LocationStart`))
  (`parent.UserConstructionScript`)
  (`|ExecutionSequence`
    (:`then_0`
      ;[1 1 1] Set trap class
      (`ChildActorComponent.SetChildActorClass` (`self.BP_ChildActor`) (`self.WeaponClass`)))
    (:`then_1`
      ;[1 1 1] Set rotation and location child actor by direction animation
      (`SceneComponent.K2_SetRelativeRotation` (`self.BP_ChildActor`) (select `/Game/plugins_addons/DeathTrapsVol_1/Blueprints/Enumeration/E_DirectionsAnimation` (`self.DirectionAnimation`) :`NewEnumerator0` _rotationstart :`NewEnumerator1` _rotationstart :`NewEnumerator2` (`self.RotationEnd`)) false false)
      (`SceneComponent.K2_SetRelativeLocation` (`self.BP_ChildActor`) (select `/Game/plugins_addons/DeathTrapsVol_1/Blueprints/Enumeration/E_DirectionsAnimation` (`self.DirectionAnimation`) :`NewEnumerator0` _locationstart :`NewEnumerator1` _locationstart :`NewEnumerator2` (`self.LocationEnd`)) false false))))